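; BP_FPCharacter is a character Blueprint that carries an AudioAnalysisComponent for musical pitch detection.
; The construction script configures the component's spectral analysis bands as a five-octave semitone range starting at C2.
; Each pitch update prints a one-frame debug message in the note's color.
; Nodes that would print note details and forward the note through CallPitchUpdate are disconnected.
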(event OnPitchUpdate(AudioAnalysisComponent)
  (params (noteName :type MusicalNoteName%20Enum :default "C") (noteColor :type Linear%20Color%20Structure) (noteNumber :type Integer))
  (Development|PrintString "Detecting pitch" true true noteColor (Utilities|Time|GetWorldDeltaSeconds)))

(event EventBeginPlay)

(event Collision|EventActorBeginOverlap
  (params (OtherActor :type Actor%20Object%20Reference)))

(event EventTick
  (params (DeltaSeconds :type Float%20%28single-precision%29)))

(fn ConstructionScript
  (Variables|/Script/VoiceOfTheOcean.AudioAnalysisComponent|SetBandSettings (Variables|Default|GetAudioAnalysisComponent) (Class|AudioMixerBlueprintLibrary|MakeMusicalSpectralAnalysisBandSettings 60 "C" 2)))