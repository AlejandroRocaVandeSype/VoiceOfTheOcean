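; Debug actor that prints live audio analysis results to the screen.
; The construction script configures the AudioAnalysis component's spectral bands as 60 semitones starting at C in octave 2.
; On BeginPlay it starts pitch detection and envelope following.
; Each update prints for a single frame: the note name and number in the note's color, or the current envelope value.
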(event OnPitchUpdate(AudioAnalysis)
  (params (noteName :type MusicalNoteName%20Enum :default "C") (noteColor :type Linear%20Color%20Structure) (noteNumber :type Integer))
  (Development|PrintString (Utilities|String|ToString(Text) (Utilities|Text|FormatText "NoteName: {a} 
NoteNumber: {b}" (Utilities|String|EnumtoString noteName) noteNumber)) true true noteColor (Utilities|Time|GetWorldDeltaSeconds)))

(event OnEnvelopeUpdate(AudioAnalysis)
  (params (EnvelopeData :type Float%20%28single-precision%29))
  (Development|PrintString (Utilities|String|ToString(Float) EnvelopeData) true true "(R=0.000000,G=0.660000,B=1.000000,A=1.000000)" (Utilities|Time|GetWorldDeltaSeconds)))

(event EventBeginPlay
  (Class|AudioAnalysisComponent|StartPitchDetection (Variables|Default|GetAudioAnalysis))
  (Class|AudioAnalysisComponent|StartEnvelopeFollowing (Variables|Default|GetAudioAnalysis)))

(event Collision|EventActorBeginOverlap
  (params (OtherActor :type Actor%20Object%20Reference)))

(event EventTick
  (params (DeltaSeconds :type Float%20%28single-precision%29)))

(fn ConstructionScript
  (Variables|/Script/VoiceOfTheOcean.AudioAnalysisComponent|SetBandSettings (Variables|Default|GetAudioAnalysis) (Class|AudioMixerBlueprintLibrary|MakeMusicalSpectralAnalysisBandSettings 60 "C" 2)))